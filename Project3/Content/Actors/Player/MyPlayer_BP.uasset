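; Player character Blueprint that handles movement, bubble scoring, a persistent high score and the game state.
; Axis inputs move it relative to control-rotation yaw, and BeginPlay loads the saved high score and sets the starting state.
; IncreaseScore adds a bubble's worth, then writes any score matching or beating the high score straight to a SaveHighscore slot, creating it if absent.
; KillPlayer and StartGame switch the GameState enum.
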(event `InputAxis|MoveForward`
  (params (AxisValue :type "Float (single-precision)"))
  ;[1 1 1] Keyboard Movement Inputs
  (`self.AddMovementInput` (`KismetMathLibrary.GetForwardVector` (`KismetMathLibrary.MakeRotator` 0.0 0.0 (.yaw (`self.GetControlRotation`)))) AxisValue))

(event `InputAxis|MoveRight`
  (params (AxisValue :type "Float (single-precision)"))
  ;[1 1 1] Keyboard Movement Inputs
  (`self.AddMovementInput` (`KismetMathLibrary.GetRightVector` (`KismetMathLibrary.MakeRotator` 0.0 0.0 (.yaw (`self.GetControlRotation`)))) AxisValue))

(event `self.ReceiveBeginPlay`
  ;[1 1 1] On start, load high score
  (`self.Load High Score`)
  (set `self.GameState` "NewEnumerator1"))

(fn `Check High Score`
  ;[1 1 1] Check if high score
  (if (>= (`self.Points`) (`self.High Score`))
    (set `self.High Score` (`self.Points`)) ; If score is higher, set as the high score
    (bind _returnvalue (`GameplayStatics.DoesSaveGameExist` (`self.Slot Name`))) ; Check for save data
    (if _returnvalue
      (bind _returnvalue_2 (`GameplayStatics.LoadGameFromSlot` (`self.Slot Name`))) ; If save data, then load
      ;[1 1 1] Set new high score in the save system
      (bind _output_get (set `self.SaverSubClass` _returnvalue_2))
      (bind _assave_highscore (cast `/Game/ScoreSystem/SaveHighscore` _output_get))
      (set `/Game/ScoreSystem/SaveHighscore.High Score` (`self.High Score`) _assave_highscore)
      (else
        (bind _returnvalue_3 (`GameplayStatics.CreateSaveGameObject` "/Game/ScoreSystem/SaveHighscore.SaveHighscore_C")) ; If no save data, then create
        (bind _output_get_2 (set `self.SaverSubClass` _returnvalue_3))
        (bind _assave_highscore_2 (cast `/Game/ScoreSystem/SaveHighscore` _output_get_2))
        (set `/Game/ScoreSystem/SaveHighscore.High Score` (`self.High Score`) _assave_highscore_2)))
    (`GameplayStatics.SaveGameToSlot` (`self.SaverSubClass`) (`self.Slot Name`)) ; Save new data to the save slot
  ))

(fn `Increase Score`
  (params (Worth :type Integer))
  ;[1 1 1] Increment Current Player Score
  (set `self.Points` (+ Worth (`self.Points`))) ; Set new score
  (`self.Check High Score`))

(fn `KillPlayer`
  (set `self.GameState` "NewEnumerator2"))

(fn `Load High Score`
  (bind _returnvalue (`GameplayStatics.DoesSaveGameExist` (`self.Slot Name`))) ; Checks for save data
  (if _returnvalue
    (bind _returnvalue_2 (`GameplayStatics.LoadGameFromSlot` (`self.Slot Name`))) ; If game data exists, load it
    (bind _output_get (set `self.SaverSubClass` _returnvalue_2))
    (bind _assave_highscore (cast `/Game/ScoreSystem/SaveHighscore` _output_get))
    (set `self.High Score` (`/Game/ScoreSystem/SaveHighscore.High Score` _assave_highscore)) ; Set player high score to save game high score
  ))

(fn `StartGame`
  (set `self.GameState` "NewEnumerator1"))

(fn `UserConstructionScript`)